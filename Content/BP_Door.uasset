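; BP_Door is a wooden door actor that swings open when the player walks into its trigger volume.
; Overlap by a BP_Player sets an OpenDoor flag that is never cleared in this Blueprint.
; While the flag is set, Tick lerps the mesh's relative rotation toward a fixed open yaw by a constant fraction each frame, giving a frame-rate-dependent ease-out.
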(event `self.Trigger.OnComponentBeginOverlap`
  (params (OverlappedComponent :type "PrimitiveComponent Object Reference") (OtherActor :type "Actor Object Reference") (OtherComp :type "PrimitiveComponent Object Reference") (OtherBodyIndex :type Integer) (bFromSweep :type Boolean) (SweepResult :type "HitResult Structure (by ref)"))
  (cast `/Game/BP_Player` OtherActor)
  (set `self.OpenDoor` true))

(event `self.ReceiveTick`
  (params (DeltaSeconds :type "Float (single-precision)"))
  (if (`self.OpenDoor`)
    (`SceneComponent.K2_SetRelativeTransform` (`self.S_Old_Wooden_Door_uflvddofa_lod3_Var1`) (`KismetMathLibrary.MakeTransform` (.location (`SceneComponent.GetRelativeTransform` (`self.S_Old_Wooden_Door_uflvddofa_lod3_Var1`))) (`KismetMathLibrary.RLerp` (.rotation (`SceneComponent.GetRelativeTransform` (`self.S_Old_Wooden_Door_uflvddofa_lod3_Var1`))) (struct :`Yaw` -90.0) 0.05) (.scale (`SceneComponent.GetRelativeTransform` (`self.S_Old_Wooden_Door_uflvddofa_lod3_Var1`)))) false false)))

(fn `UserConstructionScript`)