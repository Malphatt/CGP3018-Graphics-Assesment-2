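; BP_FiringShip is a ship actor that repeatedly fires BP_Bullet actors after a 10-second delay from the start of its life.
; Tick accumulates time alive, then runs a half-second fire timer while StopFiring is false.
; Each bullet spawns with the ship's rotation and scale at a large fixed world-space offset along negative Y from its location.
; StopFiring is only read here, never set.
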(event `self.ReceiveTick`
  (params (DeltaSeconds :type "Float (single-precision)"))
  (bind _output_get (set `self.Time Alive` (+ DeltaSeconds (`self.Time Alive`))))
  (if (< _output_get 10.0)
    _
    (elif (not (`self.Stop Firing`))
      (bind _output_get_2 (set `self.Time Since Last Fire` (+ DeltaSeconds (`self.Time Since Last Fire`))))
      (if (> _output_get_2 0.5)
        (set `self.Time Since Last Fire` 0.0)
        (`|SpawnActorFromClass` "/Game/Blueprints/BP_Bullet.BP_Bullet_C" (`KismetMathLibrary.MakeTransform` (+ (.location (`self.GetTransform`)) (0.0 -15000.0 0.0)) (.rotation (`self.GetTransform`)) (.scale (`self.GetTransform`))) "Undefined" "MultiplyWithRoot" null null)))))

(fn `UserConstructionScript`)