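; Spaceship actor that flies forward along its mesh's local Y axis, then plays a scripted destruction sequence.
; Tick moves the mesh a fixed step per frame, not scaled by delta time, until a distance threshold triggers a DoOnce.
; That enables physics, waits, then loops over "FiringShip"-tagged BP_FiringShip actors to stop their fire.
; The same loop body spawns delay-staggered explosions at four ExplosionPoint components.
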(event `self.ReceiveTick`
  (params (DeltaSeconds :type "Float (single-precision)"))
  (`SceneComponent.K2_AddLocalOffset` (`self.GC_spaceship_manticore_class`) (0.0 5.0 0.0) false false)
  (if (> (.y (.location (`SceneComponent.GetRelativeTransform` (`self.GC_spaceship_manticore_class`)))) 5000.0)
    (`/Engine/EditorBlueprintResources/StandardMacros.DoOnce` false
      (:`Completed`
        (`PrimitiveComponent.SetSimulatePhysics` (`self.GC_spaceship_manticore_class`) true)
        (`KismetSystemLibrary.Delay` 1.0)
        (bind _outactors (`GameplayStatics.GetAllActorsWithTag` "FiringShip"))
        (for _array_element _outactors
          (bind _asbp_firing_ship (cast `/Game/Blueprints/BP_FiringShip` _array_element))
          (set `/Game/Blueprints/BP_FiringShip.Stop Firing` true _asbp_firing_ship)
          (`GameplayStatics.SpawnEmitterAtLocation` "/Game/StarterContent/Particles/P_Explosion.P_Explosion" (.location (`SceneComponent.K2_GetComponentToWorld` (`self.Explosion Point 1`))) (.rotation (`SceneComponent.K2_GetComponentToWorld` (`self.Explosion Point 1`))) (.scale (`SceneComponent.K2_GetComponentToWorld` (`self.Explosion Point 1`))))
          (`KismetSystemLibrary.Delay` 0.5)
          (`GameplayStatics.SpawnEmitterAtLocation` "/Game/StarterContent/Particles/P_Explosion.P_Explosion" (.location (`SceneComponent.K2_GetComponentToWorld` (`self.Explosion Point 2`))) (.rotation (`SceneComponent.K2_GetComponentToWorld` (`self.Explosion Point 2`))) (.scale (`SceneComponent.K2_GetComponentToWorld` (`self.Explosion Point 2`))))
          (`KismetSystemLibrary.Delay` 0.8)
          (`GameplayStatics.SpawnEmitterAtLocation` "/Game/StarterContent/Particles/P_Explosion.P_Explosion" (.location (`SceneComponent.K2_GetComponentToWorld` (`self.Explosion Point 3`))) (.rotation (`SceneComponent.K2_GetComponentToWorld` (`self.Explosion Point 3`))) (.scale (`SceneComponent.K2_GetComponentToWorld` (`self.Explosion Point 3`))))
          (`KismetSystemLibrary.Delay` 1.0)
          (`GameplayStatics.SpawnEmitterAtLocation` "/Game/StarterContent/Particles/P_Explosion.P_Explosion" (.location (`SceneComponent.K2_GetComponentToWorld` (`self.Explosion Point 4`))) (.rotation (`SceneComponent.K2_GetComponentToWorld` (`self.Explosion Point 4`))) (.scale (`SceneComponent.K2_GetComponentToWorld` (`self.Explosion Point 4`)))))))))

(fn `UserConstructionScript`)