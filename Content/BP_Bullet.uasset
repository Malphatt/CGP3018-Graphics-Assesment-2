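; BP_Bullet is a bullet actor that flies in a straight line and removes itself after a set distance.
; Every Tick it offsets its Cube along local Y by a fixed step, without sweep or delta-time scaling, so speed depends on frame rate.
; Once the Cube's relative Y passes a threshold, it turns off physics simulation and destroys the actor after a short delay.
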(event `self.ReceiveTick`
  (params (DeltaSeconds :type "Float (single-precision)"))
  (`SceneComponent.K2_AddLocalOffset` (`self.Cube`) (0.0 500.0 0.0) false false)
  (if (> (.y (.location (`SceneComponent.GetRelativeTransform` (`self.Cube`)))) 30000.0)
    (`PrimitiveComponent.SetSimulatePhysics` (`self.Cube`) false)
    (`KismetSystemLibrary.Delay` 0.2)
    (`self.K2_DestroyActor`)))

(fn `UserConstructionScript`)