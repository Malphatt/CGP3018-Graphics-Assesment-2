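; Black hole actor that drives its material look and surrounds the world origin with randomly coloured stars.
; The construction script pushes disk colour, size, and direction-signed ring speed and intensity into BlackHole material parameters.
; BeginPlay spawns BP_4 stars in a random spherical shell around the origin, not the actor.
; Star tints use red- or blue-weighted random formulas; RandomInteger(2) leaves the green case unreachable.
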(event `self.ReceiveBeginPlay`
  (bind _returnvalue (`KismetMathLibrary.RandomFloatInRange` 0.0 1.0))
  (bind _returnvalue_2 (`KismetMathLibrary.RandomFloatInRange` 0.0 1.0))
  (bind _mincolourvariantmultmax (`self.MinColourVariantMultMax`))
  (bind _star_spawn_radius_start (`self.Star Spawn Radius Start`))
  (bind _mincolourvariantmultmax_2 (`self.MinColourVariantMultMax`))
  (bind _mincolourvariantmultmax_3 (`self.MinColourVariantMultMax`))
  (bind _returnvalue_3 (`KismetMathLibrary.RandomFloatInRange` (`self.MinColour`) 1.0))
  (for _ (range (+ (`self.Number of Stars`) 1))
    (bind _returnvalue_4 (`|SpawnActorFromClass` "/Game/Materials/4/BP_4.BP_4_C" (`KismetMathLibrary.Conv_VectorToTransform` (* (* (`KismetMathLibrary.RandomFloatInRange` 1.0 (+ (/ (`self.Star Spawn Radius Size`) _star_spawn_radius_start) 1.0)) (`KismetMathLibrary.RandomUnitVector`)) _star_spawn_radius_start)) "Undefined" "MultiplyWithRoot" null null))
    ;[1 1 1] Set Colour
    (switch `int` (`KismetMathLibrary.RandomInteger` 2)
      (:`0`
        (set `/Game/Materials/4/BP_4.Colour` (`KismetMathLibrary.MakeVector` _returnvalue_3 (* _returnvalue_3 (`KismetMathLibrary.RandomFloatInRange` 0.0 _mincolourvariantmultmax_2)) (* _returnvalue_3 (`KismetMathLibrary.RandomFloatInRange` 0.0 _mincolourvariantmultmax_2))) _returnvalue_4))
      (:`1`
        (set `/Game/Materials/4/BP_4.Colour` (`KismetMathLibrary.MakeVector` (* _returnvalue (`KismetMathLibrary.RandomFloatInRange` 0.0 _mincolourvariantmultmax)) (* _returnvalue (`KismetMathLibrary.RandomFloatInRange` 0.0 _mincolourvariantmultmax)) _returnvalue) _returnvalue_4))
      (:`2`
        (set `/Game/Materials/4/BP_4.Colour` (`KismetMathLibrary.MakeVector` (* _returnvalue_2 (`KismetMathLibrary.RandomFloatInRange` 0.0 _mincolourvariantmultmax_3)) _returnvalue_2 (* _returnvalue_2 (`KismetMathLibrary.RandomFloatInRange` 0.0 _mincolourvariantmultmax_3))) _returnvalue_4)))))

(fn `UserConstructionScript`
  (locals (`Base Ring Rad Intensity` :type "Float (double-precision)" :default 2.25))
  (`MeshComponent.SetVectorParameterValueOnMaterials` (`self.Black Hole`) "Accreation Disk Colour" (`self.Colour`))
  (`MeshComponent.SetScalarParameterValueOnMaterials` (`self.Black Hole`) "Black Hole Size" (`self.Size`))
  (`MeshComponent.SetScalarParameterValueOnMaterials` (`self.Black Hole`) "Ring Rotation Speed" (* (`self.Ring Speed`) (`self.Ring Direction`)))
  (`MeshComponent.SetScalarParameterValueOnMaterials` (`self.Black Hole`) "Ring Radius Intensity" (* (`local.Base Ring Rad Intensity`) (`self.Ring Direction`))))