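; BP_4 is a star actor that exposes colour, noise scale and glow power settings for the materials on its Star component.
; The construction script pushes all three values into the material parameters, so edits show in the editor.
; Tick reapplies only the colour every frame, so runtime colour changes take effect while noise and glow stay as constructed.
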(event `self.ReceiveTick`
  (params (DeltaSeconds :type "Float (single-precision)"))
  (`MeshComponent.SetVectorParameterValueOnMaterials` (`self.Star`) "Colour" (`self.Colour`)))

(fn `UserConstructionScript`
  (`MeshComponent.SetVectorParameterValueOnMaterials` (`self.Star`) "Colour" (`self.Colour`))
  (`MeshComponent.SetScalarParameterValueOnMaterials` (`self.Star`) "Noise Scale" (`self.Noise Scale`))
  (`MeshComponent.SetScalarParameterValueOnMaterials` (`self.Star`) "Glow Power" (`self.Glow Power`)))